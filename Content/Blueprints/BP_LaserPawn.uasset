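; Pawn with laser eyes that burn away actors carrying a GrabComponent when the camera looks at them.
; Each Tick, an object line trace from the camera finds targets, activates both Niagara beams at hit distance, and starts a kill timer with beam audio.
; When the timer expires, BurnActor destroys the targeted actor.
; Hitting an actor without that component stops the beams and clears the timer; a trace miss changes nothing.
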(event `self.ReceiveTick`
  (params (DeltaSeconds :type "Float (single-precision)"))
  (bind _camera (`self.Camera`))
  (bind _sc_laserbeam (`self.SC_LaserBeam`))
  (bind _currentkilltimer (`self.CurrentKillTimer`))
  (bind _returnvalue (+ (`SceneComponent.K2_GetComponentLocation` _camera) (`self.LaserOriginOffset`)))
  (bind (_outhit _returnvalue_2) (`KismetSystemLibrary.LineTraceSingleForObjects` _returnvalue (+ _returnvalue (* (`KismetMathLibrary.GetForwardVector` (`SceneComponent.K2_GetComponentRotation` _camera)) (`self.LaserExtent`))) (`|MakeArray` "ObjectTypeQuery4" "ObjectTypeQuery1" "ObjectTypeQuery2" :!type "EObjectTypeQuery Enum")))
  (if _returnvalue_2
    (bind (_bblockinghit _binitialoverlap _time _distance _location _impactpoint _normal _impactnormal _physmat _hitactor) (`GameplayStatics.BreakHitResult` _outhit))
    ;[0 0 0] Checks for Grab Component Presence
    (if (> (`KismetArrayLibrary.Array_Length` (`self.K2_GetComponentsByClass` _hitactor "/Game/VRTemplate/Blueprints/GrabComponent.GrabComponent_C")) 0)
      ;[0 0 0] Activates Lasers
      (set `self.TargetedActor` _hitactor)
      (`self.ActivateLaserEyes` (`KismetMathLibrary.VSize` (- _returnvalue _location)))
      (if (not (`KismetSystemLibrary.K2_IsTimerActiveHandle` (`self.CurrentKillTimer`)))
        (bind _returnvalue_3 (`KismetSystemLibrary.K2_SetTimer` null "BurnActor" (`self.LaserKillThreshold`)))
        (set `self.CurrentKillTimer` _returnvalue_3)
        ;[0 0 0] Plays Laser Beam SFX
        (if (not (`AudioComponent.IsPlaying` _sc_laserbeam))
          (`AudioComponent.Play` _sc_laserbeam 0.1)))
      (else
        ;[0 0 0] Deactivates Lasers & Clears Current Kill Timer
        (`self.DeactivateLaserEyes`)
        (if (`KismetSystemLibrary.K2_IsValidTimerHandle` _currentkilltimer)
          (`KismetSystemLibrary.K2_ClearAndInvalidateTimerHandle` _currentkilltimer))))))

(fn `ActivateLaserEyes`
  (params (LaserEndDistance :type "Float (double-precision)"))
  (for _array_element (`|MakeArray` (`self.NS_LaserEyes_Right`) (`self.NS_LaserEyes_Left`))
    (`ActorComponent.Activate` _array_element false)
    (`NiagaraComponent.SetVariableFloat` _array_element "User.Beam_Distance" LaserEndDistance))
  (return))

(fn `BurnActor`
  (`self.K2_DestroyActor` (`self.TargetedActor`))
  (set `self.TargetedActor` null)
  (return))

(fn `DeactivateLaserEyes`
  (for _array_element (`|MakeArray` (`self.NS_LaserEyes_Right`) (`self.NS_LaserEyes_Left`))
    (`ActorComponent.Deactivate` _array_element))
  (return))

(fn `UserConstructionScript`)