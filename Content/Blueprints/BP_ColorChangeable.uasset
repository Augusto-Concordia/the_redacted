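; BP_ColorChangeable is a component that lets its owning actor change color at runtime.
; On BeginPlay it caches the owner's root primitive component and replaces the material at a configurable slot with a dynamic instance of itself.
; ChangeColor writes the given color into a named vector parameter on that instance.
; Both steps silently do nothing when their casts fail.
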(event `self.ReceiveBeginPlay`
  (bind _materialtargetindex (`self.MaterialTargetIndex`))
  (bind _asprimitive_component (cast `PrimitiveComponent` (`Actor.RootComponent` (`self.GetOwner`))))
  (bind _output_get (set `self.RootComponent` _asprimitive_component))
  (bind _returnvalue (`PrimitiveComponent.CreateDynamicMaterialInstance` _output_get _materialtargetindex (`PrimitiveComponent.GetMaterial` _output_get _materialtargetindex) "None"))
  (`PrimitiveComponent.SetMaterial` _output_get _materialtargetindex _returnvalue))

(fn `ChangeColor`
  (params (Color :type "Vector Structure"))
  (bind _asmaterial_instance_dynamic (cast `MaterialInstanceDynamic` (`PrimitiveComponent.GetMaterial` (`self.RootComponent`) (`self.MaterialTargetIndex`))))
  (`MaterialInstanceDynamic.SetVectorParameterValue` _asmaterial_instance_dynamic (`self.ColorParameterName`) (`KismetMathLibrary.Conv_VectorToLinearColor` Color)))